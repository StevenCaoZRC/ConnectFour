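; BP_SelectorTile is a column selector on a BP_Board grid that places a piece in its column when clicked.
; Its OnClick_Multicast event briefly swaps the tile to the selected material, then restores the default after a delay.
; It then finds its own column through the board's SelectorTileArray, scans rows from the last index backwards, and calls ChangeColour on the first unoccupied play tile.
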(event `OnClick_Multicast`
  (`KismetSystemLibrary.PrintString` "MultiCast - OnClick")
  (`PrimitiveComponent.SetMaterial` (`self.TileMesh`) 0 "/Game/CustomMaterials/MaterialInstace/MI_Selector_Selected.MI_Selector_Selected")
  (`KismetSystemLibrary.Delay` 1.0)
  (`PrimitiveComponent.SetMaterial` (`self.TileMesh`) 0 "/Game/CustomMaterials/MaterialInstace/MI_Selector_Default.MI_Selector_Default")
  (bind _outactors (`GameplayStatics.GetAllActorsOfClass` "/Game/Blueprints/BP_Board.BP_Board_C"))
  (bind _output (`|GetArrayItem` _outactors))
  (bind _playtilearray_rows (break `BoardRowData` (`|GetArrayItem` (`Board.PlayTileArray_Columns` _output) (`KismetArrayLibrary.Array_Find` (`/Game/Blueprints/BP_Board.SelectorTile_Array` _output) self))))
  ;[1 1 1] (Reverse Forloop with break basically)  Goes from the bottom of the column and checks to place a tile down
  (bind _output_get (set `self.RowIndex` (`KismetArrayLibrary.Array_Length` _playtilearray_rows)))
  (while (!= _output_get 0)
    (bind _output_2 (`|GetArrayItem` _playtilearray_rows (- (`self.RowIndex`) 1)))
    (if (`BaseTile.Occupied` _output_2)
      (`/Engine/EditorBlueprintResources/StandardMacros.DecrementInt` (`self.RowIndex`))
      (else
        (`PlayTile.ChangeColour` _output_2)
        (set `self.RowIndex` 0)))))

(fn `UserConstructionScript`)