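; Player character for a networked Connect Four game that lets the player whose turn it is click selector tiles.
; The TriggerClick input traces from the mouse cursor into the world, with debug drawing and printing, looking for a selector tile.
; If the tile is interactable and the player index matches the current turn, a server event triggers that tile's multicast click.
; The FLineTrace function is an empty stub.
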(event `self.ReceiveBeginPlay`)

(event `OnClick_Server`
  (params (`Selector Reference` :type "/Game/Blueprints/BP_SelectorTile Object Reference"))
  ;[1 1 1] Event to be executed on the server
  (`/Engine/EditorBlueprintResources/StandardMacros.IsValid` `Selector Reference`
    (:`Is Valid`
      (`/Game/Blueprints/BP_SelectorTile.OnClick_Multicast` `Selector Reference`))
    (:`Is Not Valid`
      (`KismetSystemLibrary.PrintString` "Selector Reference Invalid" true true (struct :`R` 0.755208 :`B` 0.163289 :`A` 1.0) 5.0))))

(event `self.ReceiveTick`
  (params (DeltaSeconds :type "Float (single-precision)")))

(event `InputAction|TriggerClick`
  (params (Key :type "Key Structure"))
  (bind (_worldlocation _worlddirection) (`PlayerController.DeprojectMousePositionToWorld` (`GameplayStatics.GetPlayerController` 0)))
  (:`Pressed`
    (bind _outhit (`KismetSystemLibrary.LineTraceSingle` :`Start` _worldlocation :`End` (+ _worldlocation (* _worlddirection 10000.0)) :`TraceChannel` "TraceTypeQuery1" :`DrawDebugType` "ForDuration" :`TraceColor` (struct :`R` 0.033717 :`G` 0.819807 :`B` 1.0 :`A` 1.0)))
    (bind (_bblockinghit _binitialoverlap _time _distance _location _impactpoint _normal _impactnormal _physmat _hitactor) (`GameplayStatics.BreakHitResult` _outhit))
    (`KismetSystemLibrary.PrintString` (`KismetSystemLibrary.GetDisplayName` _hitactor) false)
    (bind _asbp_selector_tile (cast `/Game/Blueprints/BP_SelectorTile` _hitactor))
    (if (and (`BaseTile.CanInteract` _asbp_selector_tile) (== (`self.PlayerIndex`) (`self.CurrentPlayerIndex`)))
      (`self.OnClick_Server` _asbp_selector_tile))))

(fn `FLineTrace`
  (returns (`AsBP Base Tile` :type "/Game/Blueprints/BP_BaseTile Object Reference")))

(fn `UserConstructionScript`)