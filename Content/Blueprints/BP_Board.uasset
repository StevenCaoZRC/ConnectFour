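; Board actor for a networked Connect Four game that builds the play grid, checks for wins and drives the game UI.
; BeginPlay creates the in-game and hidden victory widgets, then only the authority spawns the selector row and tile grid for replication to clients.
; Tiles fill a C++-defined 2D array column by column.
; A server event passes the selector's current tile to C++ CheckWin, and multicast events show the winner and toggle the HUD.
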(event `self.ReceiveBeginPlay`
  ;[1 1 1] In game Widget
  (bind _asbp_connect_four_character (cast `/Game/Blueprints/BP_ConnectFourCharacter` (`GameplayStatics.GetPlayerCharacter` 0)))
  (set `self.Player` _asbp_connect_four_character)
  (bind _returnvalue (`|CreateWidget` "/Game/UserInterface/Widget_Ingame.Widget_Ingame_C" (`GameplayStatics.GetPlayerController` 0)))
  (bind _output_get (set `self.InGameWidget` _returnvalue))
  (`UserWidget.AddToViewport` _output_get 0)
  (bind _returnvalue_2 (`GameplayStatics.GetCurrentLevelName` true))
  (`self.ShowUI_MultiCast` (`KismetStringLibrary.EqualEqual_StrStr` _returnvalue_2 "Level_Main"))
  ;[1 1 1] Begin Play - Setting up initial Victory Screen
  (bind _returnvalue_3 (`|CreateWidget` "/Game/UserInterface/Widget_VictoryScreen.Widget_VictoryScreen_C" (`GameplayStatics.GetPlayerController` 0)))
  (bind _output_get_2 (set `self.VictoryScreenWidget` _returnvalue_3))
  (`UserWidget.AddToViewport` _output_get_2 0)
  (`Widget.SetVisibility` _returnvalue_3 "Hidden")
  (`Widget.SetVisibility` (`self.VictoryScreenWidget`) "Hidden")
  ;[1 1 1] Setting initial spawn locoation
  (set `self.NewSpawnLocation` (`SceneComponent.K2_GetComponentLocation` (`self.DefaultSceneRoot`)))
  ;[1 1 1] Only Server needs to spawn board as the client will replicate the board
  (`/Engine/EditorBlueprintResources/ActorMacros.Switch Has Authority`
    (:`Authority`
      (`self.Spawn Selector Row`)
      (`self.SpawningBoard`))))

(event `CheckWin_Server`
  (params (SelectorReference :type "/Game/Blueprints/BP_SelectorTile Object Reference"))
  (bind _currenttile (`/Game/Blueprints/BP_SelectorTile.CurrentTile` SelectorReference))
  (`/Engine/EditorBlueprintResources/StandardMacros.IsValid` _currenttile
    (:`Is Valid`
      ;[1 1 1] Passing in Current tile to be checked using C++ function
      (bind _returnvalue (`self.CheckWin` _currenttile))
      (if _returnvalue
        (bind _asbp_connect_four_character (cast `/Game/Blueprints/BP_ConnectFourCharacter` (`GameplayStatics.GetPlayerCharacter` 0)))
        (`self.ShowVictoryScreen_MultiCast` _asbp_connect_four_character)))
    (:`Is Not Valid`
      (`KismetSystemLibrary.PrintString` "Hello"))))

(event `ShowVictoryScreen_MultiCast`
  (params (PlayerServer :type "/Game/Blueprints/BP_ConnectFourCharacter Object Reference"))
  ;[1 1 1] Displaying Victory Screen for both players
  (bind _asbp_connect_four_character (cast `/Game/Blueprints/BP_ConnectFourCharacter` (`GameplayStatics.GetPlayerCharacter` 0)))
  (set `ConnectFourCharacter.WinnerName` (`KismetMathLibrary.SelectString` "Player 2" "Player 1" (== (`ConnectFourCharacter.CurrentPlayerIndex` _asbp_connect_four_character) 0)) _asbp_connect_four_character)
  (`Widget.SetVisibility` (`self.VictoryScreenWidget`) "Visible")
  (`self.ShowUI_MultiCast` false))

(event `ShowUI_MultiCast`
  (params (TurnOnVisibility :type Boolean))
  (bind _ingamewidget (`self.InGameWidget`))
  ;[1 1 1] MultiCast Event for showing or hiding in game UI
  (if (and TurnOnVisibility (not (`ConnectFourCharacter.WinGame` (`self.Player`))))
    (`Widget.SetVisibility` _ingamewidget "Visible")
    (else
      (`Widget.SetVisibility` _ingamewidget "Hidden"))))

(fn `Spawn Selector Row`
  (bind (_newspawnlocation_x _newspawnlocation_y _newspawnlocation_z) (`KismetMathLibrary.BreakVector` (`self.NewSpawnLocation`)))
  (bind (_newspawnlocation_x_2 _newspawnlocation_y_2 _newspawnlocation_z_2) (`KismetMathLibrary.BreakVector` (`self.NewSpawnLocation`)))
  ;[1 1 1] Calculation for Selector starting location
  (set `self.NewSpawnLocation` (`KismetMathLibrary.MakeVector` _newspawnlocation_x _newspawnlocation_y (+ _newspawnlocation_z (`self.HorizontalSpacing`) (`self.SizeOfTile`))))
  ;[1 1 1] Decremented Row length as Array starts at 0 index instead of 1
  (for _ (range (`self.NumberOfColumns`))
    (bind _returnvalue (`|SpawnActorFromClass` "/Game/Blueprints/BP_SelectorTile.BP_SelectorTile_C" (`KismetMathLibrary.MakeTransform` (`self.NewSpawnLocation`) (struct) (0.75 0.75 0.75)) "Undefined" "OverrideRootScale" null null))
    ;[1 1 1] Adding to Selector Array
    (`KismetArrayLibrary.Array_Add` (`self.SelectorTile_Array`) _returnvalue)
    (bind (_returnvalue_x _returnvalue_y) (`KismetMathLibrary.BreakVector` (`SceneComponent.K2_GetComponentLocation` (`BaseTile.TileMesh` _returnvalue))))
    (set `self.NewSpawnLocation` (`KismetMathLibrary.MakeVector` _returnvalue_x (- _returnvalue_y (+ (`self.SizeOfTile`) (`self.VerticalSpacing`))) _newspawnlocation_z_2)))
  (return))

(fn `SpawningBoard`
  (locals (LoopIndex :type Integer) (RowIndex :type Integer) (ColumnIndex :type Integer))
  (bind (_newspawnlocation_x _newspawnlocation_y) (`KismetMathLibrary.BreakVector` (`self.NewSpawnLocation`)))
  (bind (_returnvalue_x _returnvalue_y _returnvalue_z) (`KismetMathLibrary.BreakVector` (`SceneComponent.K2_GetComponentLocation` (`self.DefaultSceneRoot`))))
  (`KismetArrayLibrary.Array_Resize` (`self.PlayTileArray_Columns`) (`self.NumberOfColumns`))
  ;[1 1 1] Resetting spawn location from what was saved from spawning the selector
  (set `self.NewSpawnLocation` (`SceneComponent.K2_GetComponentLocation` (`self.DefaultSceneRoot`)))
  (for _index (range (+ (`self.BoardSize`) 1))
    ;[1 1 1] Checks if the spawning is at the end of the row, if so go to the next
    (bind _output_get (set `local.LoopIndex` _index))
    (if (and (== (mod _output_get (- (`self.NumberOfColumns`) 1)) 0) (!= _output_get 0))
      ;[1 1 1] Calculation for spawning on the next row
      (set `self.NewSpawnLocation` (`KismetMathLibrary.MakeVector` _newspawnlocation_x (- _newspawnlocation_y (+ (`self.SizeOfTile`) (`self.HorizontalSpacing`))) _returnvalue_z)))
    (bind _returnvalue (`|SpawnActorFromClass` "/Game/Blueprints/BP_PlayTile.BP_PlayTile_C" (`KismetMathLibrary.MakeTransform` (`self.NewSpawnLocation`)) "Undefined" "OverrideRootScale" null null))
    ;[1 1 1] Adding 2D array made in C++
    (`KismetArrayLibrary.Array_Add` (`.PlayTileArray_Rows` (break `BoardRowData` (`|GetArrayItem` (`self.PlayTileArray_Columns`) (`local.ColumnIndex`)))) _returnvalue)
    (set `local.RowIndex` (+ (`local.RowIndex`) 1))
    (if (== (`local.RowIndex`) 6)
      (set `local.RowIndex` 0)
      (`/Engine/EditorBlueprintResources/StandardMacros.IncrementInt` (`local.ColumnIndex`)
        (:`  `
          _)))
    (bind (_returnvalue_x_2 _returnvalue_y_2 _returnvalue_z_2) (`KismetMathLibrary.BreakVector` (`SceneComponent.K2_GetComponentLocation` (`BaseTile.TileMesh` _returnvalue))))
    (set `self.NewSpawnLocation` (`KismetMathLibrary.MakeVector` _returnvalue_x_2 _returnvalue_y_2 (- _returnvalue_z_2 (+ (`self.SizeOfTile`) (`self.VerticalSpacing`))))))
  (return))

(fn `UserConstructionScript`)